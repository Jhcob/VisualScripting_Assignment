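; BP_LightDoor is a puzzle door with a spotlight, driven by a pressure-plate overlap box.
; Beginning an overlap turns the light green and raises the door; ending one turns it red and lowers it, each as an instant offset.
; Two DoOnce nodes reset each other so the moves alternate without stacking.
; The box does not filter actors, so any end overlap closes an open door.
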(event OnComponentBeginOverlap(Box)
  (params (OverlappedComponent :type Primitive%20Component%20Object%20Reference) (OtherActor :type Actor%20Object%20Reference) (OtherComp :type Primitive%20Component%20Object%20Reference) (OtherBodyIndex :type Integer) (bFromSweep :type Boolean) (SweepResult :type Hit%20Result%20Structure%20%28by%20ref%29))
  (bind _spotlight_door (Variables|Default|GetSpotLight_Door))
  (bind _door (Variables|Default|Getdoor))
  ;[1 1 1] Pressure plate
  (Utilities|FlowControl|DoOnce false
    (:Completed
      (Rendering|Components|Light|SetLightColor _spotlight_door "(R=0.009946,G=0.343750,B=0.000000,A=1.000000)" true)
      (Utilities|FlowControl|Delay 0.0)
      (Transformation|AddLocalOffset _door "0.000000,0.000000,300.000000" false false)
      (Utilities|FlowControl|DoOnce false) ; enters at Reset
    )))

(event OnComponentEndOverlap(Box)
  (params (OverlappedComponent :type Primitive%20Component%20Object%20Reference) (OtherActor :type Actor%20Object%20Reference) (OtherComp :type Primitive%20Component%20Object%20Reference) (OtherBodyIndex :type Integer))
  (bind _spotlight_door (Variables|Default|GetSpotLight_Door))
  (bind _door (Variables|Default|Getdoor))
  ;[1 1 1] Pressure plate
  (Utilities|FlowControl|DoOnce false
    (:Completed
      (Rendering|Components|Light|SetLightColor _spotlight_door "(R=1.000000,G=0.040252,B=0.090013,A=1.000000)" true)
      (Utilities|FlowControl|Delay 0.0)
      (Transformation|AddLocalOffset _door "0.000000,0.000000,-300.000000" false false)
      (Utilities|FlowControl|DoOnce false) ; enters at Reset
    )))

(fn ConstructionScript)