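; Shooting-puzzle target that takes four hits and reports each one to PlatformGoal.
; Each overlap on Sphere destroys the next numbered sphere through a MultiGate, with a DoOnce and short delay debouncing hits.
; The first hit opens a gate, fed by Tick and TargetStart, that repeatedly nudges the mesh by random local X/Y offsets after a delay.
; The fourth hit closes that gate and leaves the DoOnce locked.
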(event OnComponentBeginOverlap(Sphere)
  (params (OverlappedComponent :type Primitive%20Component%20Object%20Reference) (OtherActor :type Actor%20Object%20Reference) (OtherComp :type Primitive%20Component%20Object%20Reference) (OtherBodyIndex :type Integer) (bFromSweep :type Boolean) (SweepResult :type Hit%20Result%20Structure%20%28by%20ref%29))
  ;[1 1 1] Hitting target
  (Utilities|FlowControl|DoOnce false :!label _label
    (:Completed
      (Class|BITarget|TargetHit(Message) (Variables|Default|GetPlatformGoal))
      (Utilities|FlowControl|MultiGate false false -1
        (:Out%200
          (Utilities|FlowControl|Sequence
            (:then_0
              (Components|DestroyComponent (Variables|Default|GetSphere1))
              (Utilities|FlowControl|Delay 0.5 :!label _label_2)
              (goto _label Reset))
            (:then_1
              ;[1 1 1] Random location
              (Utilities|FlowControl|Gate true) ; enters at Open
            )))
        (:Out%201
          (Components|DestroyComponent (Variables|Default|GetSphere2))
          (goto _label_2))
        (:Out%202
          (Components|DestroyComponent (Variables|Default|GetSphere3))
          (goto _label_2))
        (:Out%203
          ;;[0.4624 1 0.512] Goal Target
          (Components|DestroyComponent (Variables|Default|GetSphere4))
          (Utilities|FlowControl|Gate true) ; enters at Close
        )))))

(event EventTick
  (params (DeltaSeconds :type Float%20%28single-precision%29))
  ;[1 1 1] Random location
  (Utilities|FlowControl|Gate true
    (:Exit
      (Utilities|FlowControl|Delay 0.4)
      (Transformation|AddLocalOffset (Variables|Debug|GetStaticMeshComponent) (Math|Vector|MakeVector (Utilities|RandomFloat 9e+01) (Utilities|RandomFloat 9e+01) 0.0) false false))))

(event EventTargetStart
  (params (IsInside :type Boolean))
  ;[1 1 1] Start puzzle
  (if IsInside
    (Utilities|FlowControl|Delay 3.0)
    ;[1 1 1] Random location
    (Utilities|FlowControl|Gate true
      (:Exit
        (Utilities|FlowControl|Delay 0.4)
        (Transformation|AddLocalOffset (Variables|Debug|GetStaticMeshComponent) (Math|Vector|MakeVector (Utilities|RandomFloat 9e+01) (Utilities|RandomFloat 9e+01) 0.0) false false)))))

(fn ConstructionScript)