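; Shooting-puzzle platform that notifies StartPuzzle when its sphere is overlapped and rewards completed target hits.
; A non-looping MultiGate counts TargetHit calls, so the fourth triggers the puzzle-success call.
; That hit also starts chained timelines and delays that raise the Protection barrier, move the platform from its start position to a hard-coded destination, lower the barrier, then shrink and destroy the actor.
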(event OnComponentBeginOverlap(Sphere)
  (params (OverlappedComponent :type Primitive%20Component%20Object%20Reference) (OtherActor :type Actor%20Object%20Reference) (OtherComp :type Primitive%20Component%20Object%20Reference) (OtherBodyIndex :type Integer) (bFromSweep :type Boolean) (SweepResult :type Hit%20Result%20Structure%20%28by%20ref%29))
  (Class|BIOverlapInterface|OverlapTarget(Message) (Variables|Default|GetStartPuzzle)))

(event EventBeginPlay
  (Variables|Default|SetStartPosition (Transformation|GetWorldLocation (Variables|Debug|GetStaticMeshComponent))))

(event EventTargetHit
  (bind _protection (Variables|Default|GetProtection))
  (bind _protection_2 (Variables|Default|GetProtection))
  (bind _returnvalue (Transformation|GetWorldScale _protection_2))
  (bind _returnvalue_2 (Transformation|GetWorldScale _protection))
  (Utilities|FlowControl|MultiGate false false -1
    (:Out%203
      (Utilities|FlowControl|Sequence
        (:then_0
          ;[1 1 1] UI_Widget
          (Default|CallPuzzleShootingSucceed))
        (:then_1
          ;[1 1 1] Set up barrier
          (bind _newtrack_0 (Timeline|TL_scale PlayFromStart)
            (:Update
              (Transformation|SetRelativeScale3D _protection_2 (Math|Vector|MakeVector (.x _returnvalue) (.y _returnvalue) (Math|Float|Lerp (.z _returnvalue) 2e+01 _newtrack_0)))
              (Utilities|FlowControl|Delay 0.4)
              ;[1 1 1] Move action
              (bind _newtrack_0_2 (Timeline|TL_platformMovement Play)
                (:Update
                  (bind _output_get (Variables|Default|SetEndPosition "-3527.000000,3454.000000,300.000000"))
                  (Transformation|SetActorLocation (Math|Vector|Lerp(Vector) (Variables|Default|GetStartPosition) _output_get _newtrack_0_2) false false)
                  (Utilities|FlowControl|Delay 12.0)
                  ;[1 1 1] Lower Barrier
                  (bind _newtrack_0_3 (Timeline|Timeline Play)
                    (:Update
                      (Transformation|SetRelativeScale3D _protection (Math|Vector|MakeVector (.x _returnvalue_2) (.y _returnvalue_2) (Math|Float|Lerp 2e+01 0.1 _newtrack_0_3)))
                      ;[1 1 1] Destroy
                      (bind _newtrack_0_4 (Timeline|Timeline_0 Play)
                        (:Update
                          (Transformation|SetActorScale3D (Math|Vector|Lerp(Vector) "1.000000,1.000000,1.000000" "0, 0, 0" _newtrack_0_4))
                          (Utilities|FlowControl|Delay 0.75)
                          (Actor|DestroyActor))))))))))))))

(fn ConstructionScript)