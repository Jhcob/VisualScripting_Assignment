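; BP_Prism is a gameplay prop with a sphere and light that animate when something overlaps its box.
; From BeginPlay, a timeline drives the scale of SphereParent until an overlap stops it.
; The overlap, with no actor filter, starts separate timelines for SphereParent scale and PointLightweapon intensity.
; A Delay on the scale timeline's update hides the Sphere after two seconds.
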(event OnComponentBeginOverlap(Box)
  (params (OverlappedComponent :type Primitive%20Component%20Object%20Reference) (OtherActor :type Actor%20Object%20Reference) (OtherComp :type Primitive%20Component%20Object%20Reference) (OtherBodyIndex :type Integer) (bFromSweep :type Boolean) (SweepResult :type Hit%20Result%20Structure%20%28by%20ref%29))
  (Utilities|FlowControl|Sequence
    (:then_0
      (bind _newtrack_0 (Timeline|Timeline Play)
        (:Update
          (Transformation|SetRelativeScale3D (Variables|Default|GetSphereParent) _newtrack_0)
          (Utilities|FlowControl|Delay 2.0)
          (Rendering|SetVisibility (Variables|Default|GetSphere) false false))))
    (:then_1
      (bind _newtrack_0_2 (Timeline|Timeline_Light PlayFromStart)
        (:Update
          (Rendering|Components|Light|SetIntensity (Variables|Default|GetPointLightweapon) _newtrack_0_2))))
    (:then_2
      (bind _newtrack_1 (Timeline|TL_scaleLoo Stop)
        (:Update
          (Transformation|SetRelativeScale3D (Variables|Default|GetSphereParent) _newtrack_1))))))

(event EventBeginPlay
  (bind _newtrack_1 (Timeline|TL_scaleLoo Play)
    (:Update
      (Transformation|SetRelativeScale3D (Variables|Default|GetSphereParent) _newtrack_1))))

(fn ConstructionScript)