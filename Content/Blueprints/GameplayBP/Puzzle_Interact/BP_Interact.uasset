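; Interactable puzzle Blueprint where the player triggers four boxes in a fixed order to activate a target, with wall-breaking sounds.
; Each InteractFunction call advances a MultiGate that checks player overlap with the next box, though the second step's branch is always true.
; Successes light green with a sound; failures flash all red with audio, then turn white and reset the gate.
; The final success calls InteractFunction on TargetInteract, then plays delayed impact and destruction sounds.
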(event EventInteractFunction
  (bind _soundpositive (Variables|Default|GetSoundPositive))
  (bind _soundpositive_2 (Variables|Default|GetSoundPositive))
  (bind _sound_hitting_wall (Variables|Default|GetSound_Hitting_Wall))
  (Utilities|FlowControl|MultiGate false false -1 :!label _label
    (:Out%200
      (bind _returnvalue (CallFunction|OverlappingPlayer (Variables|Default|GetBox1)))
      (if _returnvalue
        ;[0.429 1 0.5083] success
        (Rendering|Material|SetMaterial (Variables|Default|Get1) 0 "/Game/Materials/M_LightMat_puzzleGREEN_Inst.M_LightMat_puzzleGREEN_Inst")
        ;[1 1 1] Audio success
        (Audio|Components|Audio|AdjustVolume _soundpositive_2 0.0 0.5 "Linear" :!class /Script/Engine.AudioComponent :!label _label_2)
        (Audio|Components|Audio|Play _soundpositive_2 0.0)
        (else
          ;[1 0.3594 0.3594] Fail _Color
          (Rendering|Material|SetMaterial (Variables|Default|Get2) 0 "/Game/Materials/M_LightMat_puzzleRED_Inst.M_LightMat_puzzleRED_Inst" :!label _label_3)
          ;[1 0.3268 0.4166] Fail_sound cue
          (AddComponent|AddAudioComponent false)
          (Utilities|FlowControl|Delay 1.0)
          ;[1 1 1] Restart Color
          (Rendering|Material|SetMaterial (Variables|Default|Get3) 0 "/Game/Materials/M_LightMat_puzzleWH_Inst.M_LightMat_puzzleWH_Inst")
          (goto _label Reset))))
    (:Out%201
      (CallFunction|OverlappingPlayer (Variables|Default|GetBox2))
      (if true
        ;[0.4106 1 0.5439] success
        (Rendering|Material|SetMaterial (Variables|Default|Get2) 0 "/Game/Materials/M_LightMat_puzzleGREEN_Inst.M_LightMat_puzzleGREEN_Inst")
        (goto _label_2)
        (else
          (goto _label_3))))
    (:Out%202
      (bind _returnvalue_2 (CallFunction|OverlappingPlayer (Variables|Default|GetBox3)))
      (if _returnvalue_2
        ;[0.4853 1 0.5363] success
        (Rendering|Material|SetMaterial (Variables|Default|Get3) 0 "/Game/Materials/M_LightMat_puzzleGREEN_Inst.M_LightMat_puzzleGREEN_Inst")
        (goto _label_2)
        (else
          (goto _label_3))))
    (:Out%203
      (bind _returnvalue_3 (CallFunction|OverlappingPlayer (Variables|Default|GetBox4)))
      (if _returnvalue_3
        ;[0.4688 1 0.5385] success
        (Rendering|Material|SetMaterial (Variables|Default|Get4) 0 "/Game/Materials/M_LightMat_puzzleGREEN_Inst.M_LightMat_puzzleGREEN_Inst")
        ;[0.5866 1 0.4762] sound cue success
        (Audio|Components|Audio|AdjustVolume _soundpositive 0.0 0.5 "Linear" :!class /Script/Engine.AudioComponent)
        (Audio|Components|Audio|Play _soundpositive 0.0)
        ;[0 1 0.2939] Execute
        (Class|BIInteractInterface|InteractFunction(Message) (Variables|Default|GetTargetInteract))
        (Utilities|FlowControl|Delay 0.2)
        ;[1 1 1 1 40] Wall
        ;;[1 1 1] Sound hitting wall
        (Audio|Components|Audio|AdjustVolume _sound_hitting_wall 1.0 1e+01 "Linear" :!class /Script/Engine.AudioComponent)
        (Audio|Components|Audio|Play _sound_hitting_wall 0.0)
        (Utilities|FlowControl|Delay 0.2)
        ;;[1 1 1] Sound breaking  wall
        (Audio|Components|Audio|AdjustVolume (Variables|Default|GetSound_destruction) 1.0 1e+01 "Linear" :!class /Script/Engine.AudioComponent)
        (Audio|Components|Audio|Play (Variables|Default|GetSound_destruction) 0.0)
        (else
          (goto _label_3))))))

(fn ConstructionScript)

(fn NewFunction)

(fn OverlappingPlayer
  (params (self2 :type Primitive%20Component%20Object%20Reference))
  (return (Collision|IsOverlappingActor self2 (Game|Player|GetPlayerPawn 0) :!class /Script/Engine.PrimitiveComponent)))

(fn NewFunction0
  (params (self2 :type Primitive%20Component%20Object%20Reference))
  (return (Collision|IsOverlappingActor self2 (Game|Player|GetPlayerPawn 0) :!class /Script/Engine.PrimitiveComponent)))