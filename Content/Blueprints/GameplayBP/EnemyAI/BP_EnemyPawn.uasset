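; BP_EnemyPawn is an enemy AI pawn that sets its maximum speed from its current alert state.
; ChangeState stores the new AlertState, maps Alert, Neutral or Investigate to a speed, and passes it to NewFunction, which writes MaxSpeed.
; A DoOnce gates the update but is reset right afterwards through ResetAlert, so later state changes still apply.
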(event Custom|ResetAlert
  (Utilities|FlowControl|DoOnce false) ; enters at Reset
)

(event EventChangeState
  (params (NewParam :type E_AlertState%20Enum :default "NewEnumerator0"))
  (Variables|Default|SetAlertState NewParam)
  (Utilities|FlowControl|DoOnce false
    (:Completed
      (CallFunction|NewFunction (Utilities|Select :Index (Variables|Default|GetAlertState) :NewEnumerator0 1e+04 :NewEnumerator1 6e+02 :NewEnumerator2 5e+03))
      (CallFunction|ResetAlert))))

(fn ConstructionScript)

(fn NewFunction
  (params (NewParam :type Float%20%28double-precision%29))
  (Variables|Default|SetMaxSpeed NewParam))